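; BP_Elevator is an elevator that moves its static mesh between its starting position and an End marker when a Pawn overlaps it.
; BeginPlay caches the start location, and a FlipFlop alternately plays and reverses a Lerp timeline that interpolates the mesh's world location without sweeping.
; A DoneMoving flag, cleared through a DoOnce on timeline update and restored on finish, blocks new triggers mid-travel.
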(event `self.ReceiveBeginPlay`
  (set `self.StartingLocation` (`SceneComponent.K2_GetComponentLocation` (`self.StaticMesh`))))

(event `self.ReceiveActorBeginOverlap`
  (params (OtherActor :type "Actor Object Reference"))
  (cast `Pawn` OtherActor)
  (if (`self.DoneMoving`)
    (`/Engine/EditorBlueprintResources/StandardMacros.FlipFlop`
      (:`A`
        (bind (_direction _newtrack_0) (`Timeline|Lerp` :!label _label)
          (:`Update`
            (`SceneComponent.K2_SetWorldLocation` (`self.StaticMesh`) (`KismetMathLibrary.VLerp` (`self.StartingLocation`) (`SceneComponent.K2_GetComponentLocation` (`self.End`)) _newtrack_0) false false)
            (`/Engine/EditorBlueprintResources/StandardMacros.DoOnce` false :!label _label_2
              (:`Completed`
                (set `self.DoneMoving` false))))
          (:`Finished`
            (set `self.DoneMoving` true)
            (goto _label_2 :!via `Reset`))))
      (:`B`
        (goto _label :!via `Reverse`)))))

(fn `UserConstructionScript`)