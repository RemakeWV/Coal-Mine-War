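; BP_TimeCard is a one-time interactable time card that the player activates while overlapping it.
; Overlap with BP_Player toggles a widget prompt and the CanInteract flag that gates Activate.
; Activate disables player input for a three-second placeholder animation (only a debug print), then restores it and destroys the box and widget.
; It finally fires the NewRT Level Blueprint event through a "ce" console command.
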(event `/Game/01_Blueprints/iInteractable.Activate`
  (params (Player :type "/Game/01_Blueprints/BP_Player Object Reference"))
  (bind _returnvalue (`PlayerCameraManager.GetOwningPlayerController` (`GameplayStatics.GetPlayerCameraManager` 0)))
  (if (`self.CanInteract?`)
    (bind _output_get (set `self.Player` Player))
    (`self.DisableInput` _output_get _returnvalue)
    (`KismetSystemLibrary.PrintString` "Playing Animation" true false (struct :`R` 0.485965 :`G` 0.071455 :`B` 1.0 :`A` 1.0) 3.0)
    (`KismetSystemLibrary.Delay` 3.0)
    (`self.EnableInput` (`self.Player`) _returnvalue)
    (`ActorComponent.K2_DestroyComponent` (`self.Box`))
    (`ActorComponent.K2_DestroyComponent` (`self.Widget`))
    (`KismetSystemLibrary.ExecuteConsoleCommand` "ce NewRT" null)))

(event `/Game/01_Blueprints/iInteractable.Deactivate`)

(event `self.ReceiveActorBeginOverlap`
  (params (OtherActor :type "Actor Object Reference"))
  (cast `/Game/01_Blueprints/BP_Player` OtherActor)
  (`SceneComponent.SetVisibility` (`self.Widget`) true false)
  (set `self.CanInteract?` true))

(event `self.ReceiveActorEndOverlap`
  (params (OtherActor :type "Actor Object Reference"))
  (cast `/Game/01_Blueprints/BP_Player` OtherActor)
  (`SceneComponent.SetVisibility` (`self.Widget`) false false)
  (set `self.CanInteract?` false))

(fn `UserConstructionScript`)