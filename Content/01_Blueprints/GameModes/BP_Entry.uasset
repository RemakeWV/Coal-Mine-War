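; BP_Entry, in the GameModes folder, runs a timed entry sequence that leads into the Museum_PutTogether level.
; On BeginPlay it plays a music cue scaled by the master and music volume settings and spawns an Item_BP in front of the player pawn.
; After a delay, it fades out the music and the camera, then opens the museum level.
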(event `self.ReceiveBeginPlay`
  (bind (_playersettingsinfo_mousespeed _playersettingsinfo_mastervolume _playersettingsinfo_effectsvolume _playersettingsinfo_voicevolume _playersettingsinfo_musicvolume) (break `/Game/01_Blueprints/Data/PlayerSettings` (`/Game/01_Blueprints/Data/BP_BFL.ReturnSettings`)))
  (bind _rootcomponent (`Actor.RootComponent` (`GameplayStatics.GetPlayerPawn` 0)))
  (bind _returnvalue (`GameplayStatics.CreateSound2D` "/Game/06_Sounds/Music/Mid-Air_Machine_-_Appalachian_Coal_Mines_120__44_01_Cue.Mid-Air_Machine_-_Appalachian_Coal_Mines_120__44_01_Cue" (* _playersettingsinfo_mastervolume _playersettingsinfo_musicvolume) 1.0 0.0 null))
  (`AudioComponent.Play` _returnvalue 0.0)
  (`|SpawnActorFromClass` "/Game/01_Blueprints/Exhibits/Item_BP.Item_BP_C" (`KismetMathLibrary.MakeTransform` (+ (`SceneComponent.K2_GetComponentLocation` _rootcomponent) (* (`SceneComponent.GetForwardVector` _rootcomponent) 420.0))) "Undefined" "OverrideRootScale" null null)
  (`KismetSystemLibrary.Delay` 10.0)
  (`AudioComponent.FadeOut` _returnvalue 5.0 0.0 "Linear")
  (`PlayerCameraManager.StartCameraFade` :`self` (`GameplayStatics.GetPlayerCameraManager` 0) :`ToAlpha` 1.0 :`Duration` 3.0 :`bHoldWhenFinished` true)
  (`KismetSystemLibrary.Delay` 5.0)
  (`GameplayStatics.OpenLevel` "Museum_PutTogether"))

(fn `UserConstructionScript`)