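; BP_Museum_PC is a player controller, apparently for a museum level, that binds key 3 to a Menu event.
; The Menu event is empty, so the key currently does nothing.
; A disconnected FlipFlop holds unfinished settings menu toggle logic: loading or saving the game, adding or removing the widget, and switching cursor and input mode.
; That logic never runs, and its MenuRef is never assigned the created widget.
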(event `Key|Three`
  (params (Key :type "Key Structure"))
  (:`Pressed`
    (`self.Menu`)))

(event `Menu`)

(fn `UserConstructionScript`)