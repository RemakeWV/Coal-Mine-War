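; BP_In-WorldMenu is an in-world menu actor that saves the game and removes itself once the player leaves its Box volume.
; When BP_Player or MotionControllerPawn ends overlap with the Box, it calls SaveGame and destroys the actor.
; An unconnected node for moving the Box to the player's capsule location never runs, and Tick is disabled.
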(event `self.ReceiveBeginPlay`
  (`parent.ReceiveBeginPlay`))

(event `self.Box.OnComponentEndOverlap`
  (params (OverlappedComponent :type "PrimitiveComponent Object Reference") (OtherActor :type "Actor Object Reference") (OtherComp :type "PrimitiveComponent Object Reference") (OtherBodyIndex :type Integer))
  (cast `/Game/01_Blueprints/BP_Player` OtherActor
    (:`then`
      (`/Game/01_Blueprints/Data/BP_BFL.SaveGame`)
      (`self.K2_DestroyActor`))
    (:`CastFailed`
      (cast `/Game/01_Blueprints/VR/MotionControllerPawn` OtherActor)
      (`/Game/01_Blueprints/Data/BP_BFL.SaveGame`)
      (`self.K2_DestroyActor`))))

(fn `UserConstructionScript`
  (`parent.UserConstructionScript`))