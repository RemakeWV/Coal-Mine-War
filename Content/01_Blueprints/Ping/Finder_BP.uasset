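; Finder_BP implements a look-to-ping system that marks what the camera points at with a world marker and a sound.
; Ping sphere-traces along the camera's forward vector; interactable BP_Items show their name, icon and color, while other hits become generic "Look" points via POI.
; PlaceMarker spawns a WorldPingActor_BP with that data, destroying the previous ping so only one exists.
; BeginPlay enables accessibility by console command; a mesh-duplicate outline highlight remains unused.
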(event `self.ReceiveBeginPlay`
  (`KismetSystemLibrary.ExecuteConsoleCommand` "Accessibility.Enable=1" null))

(fn `Ping`
  (params (Camera :type "CameraComponent Object Reference"))
  (locals (Range :type "Float (double-precision)" :default 1000000.0) (CameraRef :type "CameraComponent Object Reference"))
  (bind _returnvalue (`SceneComponent.K2_GetComponentLocation` Camera))
  ;[1 1 1] Trace out and find
  (set `local.CameraRef` Camera)
  (bind (_outhit _returnvalue_2) (`KismetSystemLibrary.SphereTraceSingle` _returnvalue (+ _returnvalue (* (`SceneComponent.GetForwardVector` Camera) (`local.Range`))) 10.0 "TraceTypeQuery1" true))
  (if _returnvalue_2
    (bind (_bblockinghit _binitialoverlap _time _distance _location _impactpoint _normal _impactnormal _physmat _hitactor) (`GameplayStatics.BreakHitResult` _outhit))
    (if (`KismetSystemLibrary.DoesImplementInterface` _hitactor "/Game/01_Blueprints/iInteractable.iInteractable_C")
      (bind (_asbp_item _bsuccess) (cast `/Game/01_Blueprints/BP_Item` _hitactor :!pure true))
      (if _bsuccess
        (bind ((`Name_14_52C0A93540AFAFE25E7B8B931BB6D475` _name) (`Icon_19_A07142C745C0D046202D4EBF2B0128BB` _icon) (`Color_22_BF75D4E9450F33B460BCBC8562DFE269` _color)) (break `/Game/01_Blueprints/ItemStruct` (`/Game/01_Blueprints/BP_Item.ItemInfo` _asbp_item)))
        (`self.PlaceMarker` (`KismetTextLibrary.Conv_StringToText` _name) (`Actor.GetDistanceTo` _asbp_item (`self.GetOwner` (`local.CameraRef`))) (`WidgetBlueprintLibrary.MakeBrushFromTexture` _icon 32 32) _location _color)
        (else
          (bind _returnvalue_3 (`|Copy` _location))
          (`self.POI` _distance _returnvalue_3 (`self.Default`) :!label _label)))
      (else
        (goto _label)))
    (`GameplayStatics.PlaySoundAtLocation` "/Game/03_Sounds/CompileSuccess_Cue.CompileSuccess_Cue" _returnvalue_3 (struct) 1.0 1.0 0.0 null null null)))

(fn `PlaceMarker`
  (params (Name :type Text) (Distance :type "Float (double-precision)") (Icon :type "SlateBrush Structure") (Location :type "Vector Structure") (Color :type "Color Structure"))
  (bind _currentping (`self.CurrentPing`)
    (:`then`
      (`Actor.K2_DestroyActor` _currentping))
    (:`else`
      _))
  (bind _returnvalue (`|SpawnActorFromClass` "/Game/01_Blueprints/Ping/WorldPingActor_BP.WorldPingActor_BP_C" (`KismetMathLibrary.MakeTransform` Location) "Undefined" "OverrideRootScale" null Name Distance Icon Location (`KismetMathLibrary.Conv_ColorToLinearColor` Color) null))
  (set `self.CurrentPing` _returnvalue))

(fn `POI`
  (params (Distance :type "Float (double-precision)") (Location :type "Vector Structure") (Color :type "Color Structure"))
  (`self.PlaceMarker` "Look" Distance (`WidgetBlueprintLibrary.MakeBrushFromTexture` "/Game/01_Blueprints/Ping/Location_ping.Location_ping") Location Color))