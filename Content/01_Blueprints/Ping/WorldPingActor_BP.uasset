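; World ping actor that shows a marker in the game world through a widget component.
; On BeginPlay it casts the component's user widget to WorldPing_BP and copies its own Location, Name, Icon and Color into it.
; The widget handles the display; the actor only supplies the data.
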(event `self.ReceiveBeginPlay`
  (bind _asworld_ping_bp (cast `/Game/01_Blueprints/Ping/WorldPing_BP` (`WidgetComponent.GetUserWidgetObject` (`self.Widget`))))
  (`self.SetValues` _asworld_ping_bp))

(fn `SetValues`
  (params (PingUI :type "/Game/01_Blueprints/Ping/WorldPing_BP Object Reference"))
  (set `/Game/01_Blueprints/Ping/WorldPing_BP.Location` (`self.Location`) PingUI)
  (set `/Game/01_Blueprints/Ping/WorldPing_BP.NameVal` (`self.Name`) PingUI)
  (set `/Game/01_Blueprints/Ping/WorldPing_BP.IconVal` (`self.Icon`) PingUI)
  (set `/Game/01_Blueprints/Ping/WorldPing_BP.Color` (`self.Color`) PingUI))

(fn `UserConstructionScript`)