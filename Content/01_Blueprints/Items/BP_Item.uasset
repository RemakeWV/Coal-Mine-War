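; BP_Item is an item actor whose mesh and mass come from a row of the ItemList data table.
; At construction it takes a random row when Random is set, otherwise the row named after its ItemType enum value.
; SetValues looks up that row, stores it in ItemInfo, and applies its mesh and a weight-based mass override to the static mesh component.
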(fn `SetValues`
  (params (RowName :type Name))
  (bind _staticmesh (`self.StaticMesh`))
  (bind _returnvalue (`|GetDataTableRow` "/Game/01_Blueprints/Items/ItemList.ItemList" RowName)
    (:`then`
      (set `self.ItemInfo` _returnvalue)
      (bind (_name _description _mesh _weight) (break `/Game/01_Blueprints/Items/ItemStruct` _returnvalue))
      (`StaticMeshComponent.SetStaticMesh` _staticmesh _mesh)
      (`PrimitiveComponent.SetMassOverrideInKg` _staticmesh "None" _weight true))))

(fn `UserConstructionScript`
  (if (`self.Random?`)
    (bind _outrownames (`DataTableFunctionLibrary.GetDataTableRowNames` "/Game/01_Blueprints/Items/ItemList.ItemList"))
    (`self.SetValues` (`|GetArrayItem` _outrownames (`KismetMathLibrary.RandomInteger` (`KismetArrayLibrary.Array_Length` _outrownames))))
    (else
      (`self.SetValues` (`KismetStringLibrary.Conv_StringToName` (`|GetEnumeratorNameAsString` (`self.ItemType`)))))))