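; BP_PickupCube is a physics cube that can be picked up and dropped.
; Pickup turns off mesh physics simulation and attaches the root to the supplied component at its current world transform.
; Drop re-enables physics and detaches the cube in place.
; The Hit event is empty, and the throttled, surface-type-based wood impact sound logic is left disconnected.
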(event `/Game/01_Blueprints/Data/PickupActorInterface.Pickup`
  (params (AttachTo :type "SceneComponent Object Reference"))
  ;[1 1 1] Pickup Event
  (`PrimitiveComponent.SetSimulatePhysics` (`self.StaticMeshComponent`) false)
  (`SceneComponent.K2_AttachToComponent` (`self.K2_GetRootComponent`) AttachTo "None" "KeepWorld" "KeepWorld" "KeepWorld" false))

(event `/Game/01_Blueprints/Data/PickupActorInterface.Drop`
  ;[1 1 1] Drop
  (`PrimitiveComponent.SetSimulatePhysics` (`self.StaticMeshComponent`) true)
  (`self.K2_DetachFromActor` "KeepWorld" "KeepWorld" "KeepWorld"))

(event `self.ReceiveHit`
  (params (MyComp :type "PrimitiveComponent Object Reference") (Other :type "Actor Object Reference") (OtherComp :type "PrimitiveComponent Object Reference") (bSelfMoved :type Boolean) (HitLocation :type "Vector Structure") (HitNormal :type "Vector Structure") (NormalImpulse :type "Vector Structure") (Hit :type "HitResult Structure (by ref)"))
  ;[1 1 1] Hit SOund
)

(fn `UserConstructionScript`)