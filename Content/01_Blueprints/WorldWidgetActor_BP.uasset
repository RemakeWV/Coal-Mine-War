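; World-space info panel actor that presents an exhibit's title, description, image and voice-over.
; The construction script looks up the Exhibit enum's name in the ExhibitList data table and stores the row, which is pushed to the InfoPanel_UI widget then and again on BeginPlay.
; Each tick it turns to face slightly above the player without pitching, and destroys itself once the player is 650 or more units away.
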(event `self.ReceiveBeginPlay`
  (bind (_info_title _info_description _info_imageinfo _info_image _info_voiceoveraudio) (break `/Game/01_Blueprints/Data/ExhibitStruct` (`self.Info`)))
  (`self.UpdateInfo` _info_title _info_description _info_imageinfo _info_image _info_voiceoveraudio))

(event `self.ReceiveTick`
  (params (DeltaSeconds :type "Float (single-precision)"))
  (bind (_returnvalue_roll _returnvalue_pitch _returnvalue_yaw) (`KismetMathLibrary.BreakRotator` (`KismetMathLibrary.FindLookAtRotation` (`self.K2_GetActorLocation`) (+ (`self.K2_GetActorLocation` (`GameplayStatics.GetPlayerPawn` 0)) (0.0 0.0 25.0)))))
  (`self.K2_SetActorRotation` (`KismetMathLibrary.MakeRotator` _returnvalue_roll 0.0 _returnvalue_yaw) true)
  (bind _asinfo_panel_ui (cast `/Game/09_UI/InfoPanel/InfoPanel_UI` (`WidgetComponent.GetUserWidgetObject` (`self.WidgetComp`))))
  (`/Engine/EditorBlueprintResources/StandardMacros.IsValid` _asinfo_panel_ui
    (:`Is Valid`
      (if (>= (`self.GetDistanceTo` (`GameplayStatics.GetPlayerCharacter` 0)) 650.0)
        (`self.K2_DestroyActor`)))))

(event `UpdateInfo`
  (params (Title :type String) (Description :type String) (PictureInfo :type String) (Image :type "Texture2D Object Reference") (Sound :type "SoundCue Object Reference"))
  (bind _asinfo_panel_ui (cast `/Game/09_UI/InfoPanel/InfoPanel_UI` (`WidgetComponent.GetUserWidgetObject` (`self.WidgetComp`))))
  (`/Game/09_UI/InfoPanel/InfoPanel_UI.UpdateTexts` _asinfo_panel_ui Title Description PictureInfo Image Sound))

(fn `UserConstructionScript`
  (bind _returnvalue (`|GetDataTableRow` "/Game/01_Blueprints/Data/ExhibitList.ExhibitList" (`KismetStringLibrary.Conv_StringToName` (`|GetEnumeratorNameAsString` (`self.Exhibit`))))
    (:`then`
      (bind _output_get (set `self.Info` _returnvalue))
      (`self.UpdateInfo` (break `/Game/01_Blueprints/Data/ExhibitStruct` _output_get) (`.Description_8_9CD18220477ACE057896FF9ACE284ED4` (break `/Game/01_Blueprints/Data/ExhibitStruct` _output_get)) (`.ImageInfo_9_F2866D2044BC17473E6496BC7E5B8ABE` (break `/Game/01_Blueprints/Data/ExhibitStruct` _output_get)) (`.Image_15_51AC237341CF8F8A520DE7A66949215A` (break `/Game/01_Blueprints/Data/ExhibitStruct` _output_get)) (`.VoiceOverAudio_18_ADF9A573431491C590ACA3AD7DA67818` (break `/Game/01_Blueprints/Data/ExhibitStruct` _output_get))))))