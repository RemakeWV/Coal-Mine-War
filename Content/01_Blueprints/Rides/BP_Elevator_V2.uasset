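; Two-stop elevator actor that carries its holder and child call buttons between a start and end point, with synchronized cab and landing doors.
; A move request either opens the doors if the cab is at that floor, or closes them, waits, and lerps to the other stop via timelines.
; Door timelines slide cab doors with the current floor's child doors, and a cancellable delay task auto-closes them.
; The construction script snaps the buttons onto their holders.
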(event `MoveElevatorEvent`
  (params (SignalPositionAtBottom :type Boolean))
  (bind _currentwaittask (`self.CurrentWaitTask`))
  ;[1 0.6562 0.6562] MoveElevatorEvent
  ;;[1 1 1] Button Press Logic
  (if (not (`self.IsMoving`))
    (if (`KismetSystemLibrary.IsValid` _currentwaittask)
      ;;;[1 1 1] Kills any previous wait task
      (`GameplayTask.EndTask` _currentwaittask))
    (if (and SignalPositionAtBottom (`self.AtBottom`))
      (`self.DoorOpen_Close`)
      ;;[1 1 1] Has doors close automatically after a time
      (bind _asynctaskproxy (`GameplayTask_WaitDelay.TaskWaitDelay` (`self.GameplayTasks`) 10.0 :!label _label)
        (:`then`
          (set `self.CurrentWaitTask` _asynctaskproxy))
        (:`OnFinish`
          (`self.DoorOpen_Close`)))
      (elif (and (not SignalPositionAtBottom) (not (`self.AtBottom`)))
        (`self.DoorOpen_Close`)
        (goto _label)
        (elif (not (`self.IsMoving`))
          (set `self.IsMoving` true)
          (`GameplayTask_WaitDelay.TaskWaitDelay` (`self.GameplayTasks`) 2.0
            (:`OnFinish`
              (if (`self.DoorsOpen`)
                ;;[1 1 1] Pre-Movement Logic
                (`KismetSystemLibrary.PrintString` "Doors are open")
                (`self.DoorOpen_Close`)
                (else
                  (`KismetSystemLibrary.PrintString` "Doors are closed")))
              (set `self.StartingPOS` (`SceneComponent.GetSocketLocation` (`self.ElevatorHolder`) "None"))
              ;;;[1 1 1] Give the player time to get in elevator
              (`GameplayTask_WaitDelay.TaskWaitDelay` (`self.GameplayTasks`) 2.0
                (:`OnFinish`
                  (if (`self.AtBottom`)
                    ;;[1 1 1] Moving To Top
                    (bind (_direction _lerpprogression) (`Timeline|Timeline_0` :!via `PlayFromStart`)
                      (:`Update`
                        (`SceneComponent.K2_SetWorldLocation` (`self.ElevatorHolder`) (`KismetMathLibrary.VLerp` (`self.StartingPOS`) (`KismetMathLibrary.TransformLocation` (`self.GetTransform`) (`self.EndPoint`)) _lerpprogression) false false)
                        (`self.K2_SetActorLocation` (`self.ChildButtonA`) (`SceneComponent.K2_GetComponentLocation` (`self.ButtonHolderA`)) false false)
                        (`self.K2_SetActorLocation` (`self.ChildButtonB`) (`SceneComponent.K2_GetComponentLocation` (`self.ButtonHolderB`)) false false)
                        (set `self.IsMoving` true))
                      (:`Finished`
                        (set `self.IsMoving` false)
                        (set `self.AtBottom` false)
                        (`AudioComponent.Play` (`self.Audio`) 0.0)
                        (`self.DoorOpen_Close`)
                        (bind _asynctaskproxy_2 (`GameplayTask_WaitDelay.TaskWaitDelay` (`self.GameplayTasks`) 10.0)
                          (:`then`
                            (set `self.CurrentWaitTask` _asynctaskproxy_2))
                          (:`OnFinish`
                            (`self.DoorOpen_Close`)))))
                    (else
                      ;;[1 1 1] Moving To Bottom
                      (bind (_direction_2 _lerpprogression_2) (`Timeline|Timeline_2` :!via `PlayFromStart`)
                        (:`Update`
                          (`SceneComponent.K2_SetWorldLocation` (`self.ElevatorHolder`) (`KismetMathLibrary.VLerp` (`self.StartingPOS`) (`KismetMathLibrary.TransformLocation` (`self.GetTransform`) (`self.StartPoint`)) _lerpprogression_2) false false)
                          (`self.K2_SetActorLocation` (`self.ChildButtonA`) (`SceneComponent.K2_GetComponentLocation` (`self.ButtonHolderA`)) false false)
                          (`self.K2_SetActorLocation` (`self.ChildButtonB`) (`SceneComponent.K2_GetComponentLocation` (`self.ButtonHolderB`)) false false)
                          (set `self.IsMoving` true))
                        (:`Finished`
                          (set `self.AtBottom` true)
                          (set `self.IsMoving` false)
                          (`AudioComponent.Play` (`self.Audio`) 0.0)
                          (`self.DoorOpen_Close`)
                          (bind _asynctaskproxy_3 (`GameplayTask_WaitDelay.TaskWaitDelay` (`self.GameplayTasks`) 10.0)
                            (:`then`
                              (set `self.CurrentWaitTask` _asynctaskproxy_3))
                            (:`OnFinish`
                              (`self.DoorOpen_Close`))))))))))))))))

(event `DoorOpen_Close`
  (bind _childdoorbottom (`self.ChildDoorBottom`))
  (bind _childdoortop (`self.ChildDoorTop`))
  (bind _childdoorbottom_2 (`self.ChildDoorBottom`))
  (bind _childdoortop_2 (`self.ChildDoorTop`))
  ;[0.7625 1 0.7292] Door Open Close Event
  (if (`self.DoorsActive`)
    (if (`self.IsMoving`)
      _)
    (else
      (set `self.DoorsActive` true)
      (if (`self.DoorsOpen`)
        ;;[1 1 1] Closing Doors
        (bind (_direction _lerpprog) (`Timeline|DoorClose` :!via `PlayFromStart`)
          (:`Update`
            (set `self.DoorsOpen` false)
            (`SceneComponent.K2_SetWorldLocation` (`self.DoorL`) (`KismetMathLibrary.VLerp` (`SceneComponent.K2_GetComponentLocation` (`self.DoorL_Out`)) (`SceneComponent.K2_GetComponentLocation` (`self.DoorL_In`)) _lerpprog) false false)
            (`SceneComponent.K2_SetWorldLocation` (`self.DoorR`) (`KismetMathLibrary.VLerp` (`SceneComponent.K2_GetComponentLocation` (`self.DoorR_Out`)) (`SceneComponent.K2_GetComponentLocation` (`self.DoorR_In`)) _lerpprog) false false)
            ;;;[1 1 1] Checks which set of doors to open
            (if (`self.AtBottom`)
              (`SceneComponent.K2_SetWorldLocation` (`/Game/01_Blueprints/Rides/BP_ElevatorDoors.DoorL` _childdoorbottom) (`KismetMathLibrary.VLerp` (`SceneComponent.K2_GetComponentLocation` (`/Game/01_Blueprints/Rides/BP_ElevatorDoors.DoorL_Out` _childdoorbottom)) (`SceneComponent.K2_GetComponentLocation` (`/Game/01_Blueprints/Rides/BP_ElevatorDoors.DoorL_In` _childdoorbottom)) _lerpprog) false false)
              (`SceneComponent.K2_SetWorldLocation` (`/Game/01_Blueprints/Rides/BP_ElevatorDoors.DoorR` _childdoorbottom) (`KismetMathLibrary.VLerp` (`SceneComponent.K2_GetComponentLocation` (`/Game/01_Blueprints/Rides/BP_ElevatorDoors.DoorR_Out` _childdoorbottom)) (`SceneComponent.K2_GetComponentLocation` (`/Game/01_Blueprints/Rides/BP_ElevatorDoors.DoorR_In` _childdoorbottom)) _lerpprog) false false)
              (else
                (`SceneComponent.K2_SetWorldLocation` (`/Game/01_Blueprints/Rides/BP_ElevatorDoors.DoorL` _childdoortop_2) (`KismetMathLibrary.VLerp` (`SceneComponent.K2_GetComponentLocation` (`/Game/01_Blueprints/Rides/BP_ElevatorDoors.DoorL_Out` _childdoortop_2)) (`SceneComponent.K2_GetComponentLocation` (`/Game/01_Blueprints/Rides/BP_ElevatorDoors.DoorL_In` _childdoortop_2)) _lerpprog) false false)
                (`SceneComponent.K2_SetWorldLocation` (`/Game/01_Blueprints/Rides/BP_ElevatorDoors.DoorR` _childdoortop_2) (`KismetMathLibrary.VLerp` (`SceneComponent.K2_GetComponentLocation` (`/Game/01_Blueprints/Rides/BP_ElevatorDoors.DoorR_Out` _childdoortop_2)) (`SceneComponent.K2_GetComponentLocation` (`/Game/01_Blueprints/Rides/BP_ElevatorDoors.DoorR_In` _childdoortop_2)) _lerpprog) false false))))
          (:`Finished`
            (`KismetSystemLibrary.PrintString` "Door closed")
            (set `self.DoorsOpen` false)
            (set `self.DoorsActive` false)))
        (else
          ;;[1 1 1] Opoening Doors
          (bind (_direction_2 _lerpval) (`Timeline|DoorOpen` :!via `PlayFromStart`)
            (:`Update`
              (set `self.DoorsOpen` true)
              (`SceneComponent.K2_SetWorldLocation` (`self.DoorL`) (`KismetMathLibrary.VLerp` (`SceneComponent.K2_GetComponentLocation` (`self.DoorL_In`)) (`SceneComponent.K2_GetComponentLocation` (`self.DoorL_Out`)) _lerpval) false false)
              (`SceneComponent.K2_SetWorldLocation` (`self.DoorR`) (`KismetMathLibrary.VLerp` (`SceneComponent.K2_GetComponentLocation` (`self.DoorR_In`)) (`SceneComponent.K2_GetComponentLocation` (`self.DoorR_Out`)) _lerpval) false false)
              ;;;[1 1 1] Checks which set of doors to open
              (if (`self.AtBottom`)
                (`SceneComponent.K2_SetWorldLocation` (`/Game/01_Blueprints/Rides/BP_ElevatorDoors.DoorL` _childdoorbottom_2) (`KismetMathLibrary.VLerp` (`SceneComponent.K2_GetComponentLocation` (`/Game/01_Blueprints/Rides/BP_ElevatorDoors.DoorL_In` _childdoorbottom_2)) (`SceneComponent.K2_GetComponentLocation` (`/Game/01_Blueprints/Rides/BP_ElevatorDoors.DoorL_Out` _childdoorbottom_2)) _lerpval) false false)
                (`SceneComponent.K2_SetWorldLocation` (`/Game/01_Blueprints/Rides/BP_ElevatorDoors.DoorR` _childdoorbottom_2) (`KismetMathLibrary.VLerp` (`SceneComponent.K2_GetComponentLocation` (`/Game/01_Blueprints/Rides/BP_ElevatorDoors.DoorR_In` _childdoorbottom_2)) (`SceneComponent.K2_GetComponentLocation` (`/Game/01_Blueprints/Rides/BP_ElevatorDoors.DoorR_Out` _childdoorbottom_2)) _lerpval) false false)
                (else
                  (`SceneComponent.K2_SetWorldLocation` (`/Game/01_Blueprints/Rides/BP_ElevatorDoors.DoorL` _childdoortop) (`KismetMathLibrary.VLerp` (`SceneComponent.K2_GetComponentLocation` (`/Game/01_Blueprints/Rides/BP_ElevatorDoors.DoorL_In` _childdoortop)) (`SceneComponent.K2_GetComponentLocation` (`/Game/01_Blueprints/Rides/BP_ElevatorDoors.DoorL_Out` _childdoortop)) _lerpval) false false)
                  (`SceneComponent.K2_SetWorldLocation` (`/Game/01_Blueprints/Rides/BP_ElevatorDoors.DoorR` _childdoortop) (`KismetMathLibrary.VLerp` (`SceneComponent.K2_GetComponentLocation` (`/Game/01_Blueprints/Rides/BP_ElevatorDoors.DoorR_In` _childdoortop)) (`SceneComponent.K2_GetComponentLocation` (`/Game/01_Blueprints/Rides/BP_ElevatorDoors.DoorR_Out` _childdoortop)) _lerpval) false false))))
            (:`Finished`
              (`KismetSystemLibrary.PrintString` "Door Opened")
              (bind _output_get (set `self.DoorsOpen` true))
              (if _output_get
                (`KismetSystemLibrary.PrintString` "Open doors"))
              (set `self.DoorsActive` false))))))))

(fn `UserConstructionScript`
  (bind _childbuttona (`self.ChildButtonA`))
  (bind _childbuttonb (`self.ChildButtonB`))
  ;[1 1 1] Set the blueprint buttons to be perfectly on the holders so that they don't jump on launch
  (`/Engine/EditorBlueprintResources/StandardMacros.IsValid` _childbuttona
    (:`Is Valid`
      (`self.K2_SetActorLocation` _childbuttona (`SceneComponent.K2_GetComponentLocation` (`self.ButtonHolderA`)) false false)
      (`/Engine/EditorBlueprintResources/StandardMacros.IsValid` _childbuttonb
        (:`Is Valid`
          (`self.K2_SetActorLocation` _childbuttonb (`SceneComponent.K2_GetComponentLocation` (`self.ButtonHolderB`)) false false))))))