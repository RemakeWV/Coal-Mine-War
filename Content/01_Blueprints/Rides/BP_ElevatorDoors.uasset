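; BP_ElevatorDoors is a doors actor for the elevator ride that positions itself at one end of a linked BP_Elevator_V2.
; Its construction script transforms the elevator's local EndPoint or StartPoint into world space, chosen by the TopElevator flag, and moves the actor there.
; Only location is set, and the event graph holds no active logic, so this Blueprint does not animate the doors itself.
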(fn `UserConstructionScript`
  (if (`KismetSystemLibrary.IsValid` (`self.Elevator`))
    (bind _asbp_elevator_v2 (cast `/Game/01_Blueprints/Rides/BP_Elevator_V2` (`self.Elevator`)))
    (if (`self.TopElevator`)
      (bind _returnvalue (`self.GetTransform` _asbp_elevator_v2))
      (`self.K2_SetActorLocation` (`KismetMathLibrary.TransformLocation` _returnvalue (`/Game/01_Blueprints/Rides/BP_Elevator_V2.EndPoint` _asbp_elevator_v2)))
      (else
        (`self.K2_SetActorLocation` (`KismetMathLibrary.TransformLocation` _returnvalue (`/Game/01_Blueprints/Rides/BP_Elevator_V2.StartPoint` _asbp_elevator_v2)))))))