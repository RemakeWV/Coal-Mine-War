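; Museum-style exhibit item that shows a child InfoPanelActor with the details of its exhibit.
; On BeginPlay it turns its ExhibitInfo enum into a row name, looks it up in the ExhibitList data table and pushes title, description and images to the panel.
; Activate and Deactivate are identical: each plays a glass impact sound and toggles the panel's visibility rather than setting it explicitly.
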(event `self.ReceiveBeginPlay`
  ;[1 1 1] Begin Play
  (`self.InitializeFromList` (`KismetStringLibrary.Conv_StringToName` (`|GetEnumeratorNameAsString` (`self.ExhibitInfo`)))))

(event `InitializeFromList`
  (params (RowName :type Name))
  ;[1 1 1] Initialize
  (bind _returnvalue (`|GetDataTableRow` "/Game/01_Blueprints/Data/ExhibitList.ExhibitList" RowName)
    (:`then`
      (bind _asinfo_panel_actor (cast `/Game/09_UI/TESTUI/InfoPanelActor` (`ChildActorComponent.ChildActor` (`self.ChildActor`))))
      (bind (_title _description _imageinfo _image) (break `/Game/01_Blueprints/Data/ExhibitStruct` _returnvalue))
      (`/Game/09_UI/TESTUI/InfoPanelActor.UpdateInfo` _asinfo_panel_actor _title _description _imageinfo _image))))

(event `/Game/01_Blueprints/Data/iInteractable.Activate`
  (params (Player :type "/Game/01_Blueprints/BP_Player Object Reference"))
  ;[1 1 1] Activate
  (`GameplayStatics.PlaySound2D` "/Game/06_Sounds/GlassImpact01_Cue.GlassImpact01_Cue" 1.0 1.0 0.0 null null)
  (`SceneComponent.ToggleVisibility` (`self.ChildActor`) false))

(event `/Game/01_Blueprints/Data/iInteractable.Deactivate`
  ;[1 1 1] Deactive
  (`GameplayStatics.PlaySound2D` "/Game/06_Sounds/GlassImpact01_Cue.GlassImpact01_Cue" 1.0 1.0 0.0 null null)
  (`SceneComponent.ToggleVisibility` (`self.ChildActor`) false))

(fn `UserConstructionScript`)