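; Wall-mounted exhibit actor that displays a framed picture with a nameplate and a toggleable info widget.
; An enum-selected ExhibitList row fills the child widget actor, image and title.
; The construction script sizes the skeletal frame with morph targets, raises it off the floor, aligns it to the wall via sphere trace, and applies the image through a dynamic material.
; Activate and Deactivate toggle the widget with sound and animation calls.
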(event `InitializeFromList`
  (params (RowName :type Name))
  (bind _returnvalue (`|GetDataTableRow` "/Game/01_Blueprints/Data/ExhibitList.ExhibitList" RowName)
    (:`then`
      (bind _asworld_widget_actor_bp (cast `/Game/01_Blueprints/WorldWidgetActor_BP` (`ChildActorComponent.ChildActor` (`self.Widget`))))
      (bind (_title _description _imageinfo _image) (break `/Game/01_Blueprints/Data/ExhibitStruct` _returnvalue))
      (`/Game/01_Blueprints/WorldWidgetActor_BP.UpdateInfo` _asworld_widget_actor_bp _title _description _imageinfo _image null)
      (set `self.Image` _image)
      (set `self.Name` _title))))

(event `self.ReceiveBeginPlay`
  (`self.SetMorphTargets` (`self.Width`) (`self.Height`))
  (`self.InitializeFromList` (`KismetStringLibrary.Conv_StringToName` (`|GetEnumeratorNameAsString` (`self.ExhibitInfo`))))
  (`self.UpdateNameplate`))

(event `SetMorphTargets`
  (params (Width :type "Float (double-precision)") (Height :type "Float (double-precision)"))
  (`SkeletalMeshComponent.SetMorphTarget` (`self.SK_PictureFrame`) "Width" Width true)
  (`SkeletalMeshComponent.SetMorphTarget` (`self.SK_PictureFrame`) "Height" Height true))

(event `self.Activate`
  (params (Player :type "/Game/01_Blueprints/BP_Player Object Reference"))
  (`GameplayStatics.PlaySound2D` "/Game/06_Sounds/GlassImpact01_Cue.GlassImpact01_Cue" 1.0 1.0 0.0 null null)
  (`SceneComponent.SetVisibility` (`self.Widget`) true false)
  (set `self.Active?` true)
  (bind _asworld_widget_actor_bp (cast `/Game/01_Blueprints/WorldWidgetActor_BP` (`ChildActorComponent.ChildActor` (`self.Widget`))))
  (bind _astest_widget (cast `/Game/09_UI/TESTUI/TestWidget` (`WidgetComponent.GetUserWidgetObject` (`/Game/01_Blueprints/WorldWidgetActor_BP.WidgetComp` _asworld_widget_actor_bp))))
  (`/Game/09_UI/TESTUI/TestWidget.PlayAnimUp` _astest_widget))

(event `self.Deactivate`
  (`GameplayStatics.PlaySound2D` "/Game/06_Sounds/GlassImpact01_Cue.GlassImpact01_Cue" 1.0 1.0 0.0 null null)
  (`SceneComponent.SetVisibility` (`self.Widget`) false false)
  (set `self.Active?` false)
  (bind _asworld_widget_actor_bp (cast `/Game/01_Blueprints/WorldWidgetActor_BP` (`ChildActorComponent.ChildActor` (`self.Widget`))))
  (bind _astest_widget (cast `/Game/09_UI/TESTUI/TestWidget` (`WidgetComponent.GetUserWidgetObject` (`/Game/01_Blueprints/WorldWidgetActor_BP.WidgetComp` _asworld_widget_actor_bp))))
  (`/Game/09_UI/TESTUI/TestWidget.PlayAnimDown` _astest_widget))

(event `UpdateNameplate`
  (bind _asnameplate_ui (cast `/Game/09_UI/Nameplate_UI` (`WidgetComponent.GetUserWidgetObject` (`self.Nameplate`))))
  (set `/Game/09_UI/Nameplate_UI.Name` (`KismetTextLibrary.Conv_StringToText` (`self.Name`)) _asnameplate_ui))

(fn `ChangeAssets`
  (params (NewMesh :type "StaticMesh Object Reference") (Picture :type Boolean)))

(fn `UserConstructionScript`
  (bind (_returnvalue_x _returnvalue_y _returnvalue_z) (`KismetMathLibrary.BreakVector` (`self.K2_GetActorLocation`)))
  (bind _image (`self.Image`))
  (bind _returnvalue (`SceneComponent.K2_GetComponentLocation` (`self.SK_PictureFrame`)))
  (bind _asmaterial_instance_dynamic (cast `MaterialInstanceDynamic` (`PrimitiveComponent.GetMaterial` (`self.Plane`) 0) :!pure true))
  (`self.InitializeFromList` (`KismetStringLibrary.Conv_StringToName` (`|GetEnumeratorNameAsString` (`self.ExhibitInfo`))))
  (set `self.Refresh` false)
  (`self.SetMorphTargets` (`self.Width`) (`self.Height`))
  ;[1 1 1] Create and set the material of this object to use later. This will be how we actually apply the texture to the same material without have a seperate material for each painting option.
  (bind _returnvalue_2 (`PrimitiveComponent.CreateDynamicMaterialInstance` (`self.Plane`) 0 (`PrimitiveComponent.GetMaterial` (`self.Plane`) 0) "None"))
  (bind _output_get (set `self.Material` _returnvalue_2))
  (`PrimitiveComponent.SetMaterial` (`self.Plane`) 0 _output_get)
  ;[1 1 1] Offest the height of the mesh by the desired height of each painting
  (`SceneComponent.K2_SetWorldLocation` (`self.SK_PictureFrame`) (`KismetMathLibrary.MakeVector` _returnvalue_x _returnvalue_y (+ _returnvalue_z (`self.DistanceFromFloor`))) false false)
  ;[1 1 1] Trace out from the center of the mesh to get the surface normal of the impact (multiply by -1 to inverse and set that as the new world Rotation of the mesh.
  (bind _outhit (`KismetSystemLibrary.SphereTraceSingle` _returnvalue _returnvalue 5.0 "TraceTypeQuery1" true))
  (`SceneComponent.K2_SetWorldRotation` (`self.SK_PictureFrame`) (`KismetMathLibrary.Conv_VectorToRotator` (* (`.ImpactNormal` (`GameplayStatics.BreakHitResult` _outhit)) -1.0)) true true)
  ;[1 1 1] Set scale of item in frame
  (`SceneComponent.SetRelativeScale3D` (`self.Plane`) (1.75 1.75 1.75))
  ;[1 1 1] For now - swap out the texture parameter of the dynamic material instance with a new texture.
  (switch `/Game/01_Blueprints/Exhibits/Wall-Item` (`self.Type`)
    (:`NewEnumerator0`
      (`self.ChangeAssets` "/Game/07_Props/PictureFrame/PictureFrame.PictureFrame" true)
      (switch `/Game/01_Blueprints/Exhibits/Options` (`self.Variations`)
        (:`NewEnumerator0`
          (`MaterialInstanceDynamic.SetTextureParameterValue` _asmaterial_instance_dynamic "Picture" _image))
        (:`NewEnumerator1`
          (`MaterialInstanceDynamic.SetTextureParameterValue` _asmaterial_instance_dynamic "Picture" _image)))
      (`self.UpdateNameplate`))))