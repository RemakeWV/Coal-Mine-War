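; Exhibit platform actor whose size is set by Width, Depth and Height morph targets on its Platform mesh.
; The construction script and BeginPlay both pass the size variables to a shared SetMorphTargets event, with Width and Depth swapped.
; The construction script also resets a Refresh flag to false on each run.
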(event `self.ReceiveBeginPlay`
  (`self.SetMorphTargets` (`self.Depth`) (`self.Width`) (`self.Height`)))

(event `SetMorphTargets`
  (params (Width :type "Float (double-precision)") (Depth :type "Float (double-precision)") (Height :type "Float (double-precision)"))
  (bind _platform (`self.Platform`))
  (`SkeletalMeshComponent.SetMorphTarget` _platform "Width" Width true)
  (`SkeletalMeshComponent.SetMorphTarget` _platform "Depth" Depth true)
  (`SkeletalMeshComponent.SetMorphTarget` _platform "Height" Height true))

(fn `UserConstructionScript`
  (set `self.Refresh` false)
  (`self.SetMorphTargets` (`self.Depth`) (`self.Width`) (`self.Height`)))