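; Two-stop elevator actor that travels between StartPoint and EndPoint and toggles its doors when MoveElevatorEvent receives a bottom or top signal.
; Timelines lerp the cab between the actor-relative points, moving child buttons along and playing audio on arrival.
; Door timelines slide the cab doors in sync with the current floor's child doors.
; A stored delay task re-toggles the doors after a wait and is cancelled by each new signal.
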(event `MoveElevatorEvent`
  (params (SignalPositionAtBottom :type Boolean))
  (bind _currentwaittask (`self.CurrentWaitTask`))
  ;[1 0.6562 0.6562] MoveElevatorEvent
  ;;[1 1 1] Button Press Logic
  (if (`KismetSystemLibrary.IsValid` _currentwaittask)
    (`GameplayTask.EndTask` _currentwaittask))
  (if (and SignalPositionAtBottom (`self.AtBottom`))
    (`KismetSystemLibrary.PrintString` "Elevator Already here!")
    (`self.DoorOpen_Close`)
    (bind _asynctaskproxy (`GameplayTask_WaitDelay.TaskWaitDelay` (`self.GameplayTasks`) 10.0 :!label _label)
      (:`then`
        (set `self.CurrentWaitTask` _asynctaskproxy))
      (:`OnFinish`
        (`self.DoorOpen_Close`)))
    (elif (and (not SignalPositionAtBottom) (not (`self.AtBottom`)))
      (`KismetSystemLibrary.PrintString` "Already here!")
      (`self.DoorOpen_Close`)
      (goto _label)
      (elif (`self.IsMoving`)
        (`KismetSystemLibrary.PrintString` "Is currently moving!")
        (else
          (if (`self.DoorsOpen`)
            ;;[1 1 1] Pre-Movement Logic
            (`self.DoorOpen_Close`))
          (set `self.StartingPOS` (`SceneComponent.GetSocketLocation` (`self.ElevatorHolder`) "None"))
          (`GameplayTask_WaitDelay.TaskWaitDelay` (`self.GameplayTasks`) 2.0
            (:`OnFinish`
              (if (`self.AtBottom`)
                ;;[1 1 1] Moving To Top
                (bind (_direction _lerpprogression) (`Timeline|Timeline_0` :!via `PlayFromStart`)
                  (:`Update`
                    (`SceneComponent.K2_SetWorldLocation` (`self.ElevatorHolder`) (`KismetMathLibrary.VLerp` (`self.StartingPOS`) (`KismetMathLibrary.TransformLocation` (`self.GetTransform`) (`self.EndPoint`)) _lerpprogression) false false)
                    (`self.K2_SetActorLocation` (`self.ChildButtonA`) (`SceneComponent.K2_GetComponentLocation` (`self.ButtonHolderA`)) false false)
                    (`self.K2_SetActorLocation` (`self.ChildButtonB`) (`SceneComponent.K2_GetComponentLocation` (`self.ButtonHolderB`)) false false)
                    (set `self.IsMoving` true))
                  (:`Finished`
                    (set `self.IsMoving` false)
                    (set `self.AtBottom` false)
                    (`AudioComponent.Play` (`self.Audio`) 0.0)
                    (`self.DoorOpen_Close`)
                    (bind _asynctaskproxy_2 (`GameplayTask_WaitDelay.TaskWaitDelay` (`self.GameplayTasks`) 10.0)
                      (:`then`
                        (set `self.CurrentWaitTask` _asynctaskproxy_2))
                      (:`OnFinish`
                        (`self.DoorOpen_Close`)))))
                (else
                  ;;[1 1 1] Moving To Bottom
                  (bind (_direction_2 _lerpprogression_2) (`Timeline|Timeline_2` :!via `PlayFromStart`)
                    (:`Update`
                      (`SceneComponent.K2_SetWorldLocation` (`self.ElevatorHolder`) (`KismetMathLibrary.VLerp` (`self.StartingPOS`) (`KismetMathLibrary.TransformLocation` (`self.GetTransform`) (`self.StartPoint`)) _lerpprogression_2) false false)
                      (`self.K2_SetActorLocation` (`self.ChildButtonA`) (`SceneComponent.K2_GetComponentLocation` (`self.ButtonHolderA`)) false false)
                      (`self.K2_SetActorLocation` (`self.ChildButtonB`) (`SceneComponent.K2_GetComponentLocation` (`self.ButtonHolderB`)) false false)
                      (set `self.IsMoving` true))
                    (:`Finished`
                      (set `self.AtBottom` true)
                      (set `self.IsMoving` false)
                      (`AudioComponent.Play` (`self.Audio`) 0.0)
                      (`self.DoorOpen_Close`)
                      (bind _asynctaskproxy_3 (`GameplayTask_WaitDelay.TaskWaitDelay` (`self.GameplayTasks`) 10.0)
                        (:`then`
                          (set `self.CurrentWaitTask` _asynctaskproxy_3))
                        (:`OnFinish`
                          (`self.DoorOpen_Close`))))))))))))))

(event `DoorOpen_Close`
  (bind _childdoorbottom (`self.ChildDoorBottom`))
  (bind _childdoortop (`self.ChildDoorTop`))
  (bind _childdoorbottom_2 (`self.ChildDoorBottom`))
  (bind _childdoortop_2 (`self.ChildDoorTop`))
  ;[0.7625 1 0.7292] Door Open Close Event
  (if (`self.DoorsOpen`)
    ;;[1 1 1] Closing Doors
    (bind (_direction _lerpprog) (`Timeline|DoorClose` :!via `PlayFromStart`)
      (:`Update`
        (`SceneComponent.K2_SetWorldLocation` (`self.DoorL`) (`KismetMathLibrary.VLerp` (`SceneComponent.K2_GetComponentLocation` (`self.DoorL_Out`)) (`SceneComponent.K2_GetComponentLocation` (`self.DoorL_In`)) _lerpprog) false false)
        (`SceneComponent.K2_SetWorldLocation` (`self.DoorR`) (`KismetMathLibrary.VLerp` (`SceneComponent.K2_GetComponentLocation` (`self.DoorR_Out`)) (`SceneComponent.K2_GetComponentLocation` (`self.DoorR_In`)) _lerpprog) false false)
        (if (`self.AtBottom`)
          (`SceneComponent.K2_SetWorldLocation` (`/Game/01_Blueprints/BP_ElevatorDoors.DoorL` _childdoorbottom) (`KismetMathLibrary.VLerp` (`SceneComponent.K2_GetComponentLocation` (`/Game/01_Blueprints/BP_ElevatorDoors.DoorL_Out` _childdoorbottom)) (`SceneComponent.K2_GetComponentLocation` (`/Game/01_Blueprints/BP_ElevatorDoors.DoorL_In` _childdoorbottom)) _lerpprog) false false)
          (`SceneComponent.K2_SetWorldLocation` (`/Game/01_Blueprints/BP_ElevatorDoors.DoorR` _childdoorbottom) (`KismetMathLibrary.VLerp` (`SceneComponent.K2_GetComponentLocation` (`/Game/01_Blueprints/BP_ElevatorDoors.DoorR_Out` _childdoorbottom)) (`SceneComponent.K2_GetComponentLocation` (`/Game/01_Blueprints/BP_ElevatorDoors.DoorR_In` _childdoorbottom)) _lerpprog) false false)
          (else
            (`SceneComponent.K2_SetWorldLocation` (`/Game/01_Blueprints/BP_ElevatorDoors.DoorL` _childdoortop_2) (`KismetMathLibrary.VLerp` (`SceneComponent.K2_GetComponentLocation` (`/Game/01_Blueprints/BP_ElevatorDoors.DoorL_Out` _childdoortop_2)) (`SceneComponent.K2_GetComponentLocation` (`/Game/01_Blueprints/BP_ElevatorDoors.DoorL_In` _childdoortop_2)) _lerpprog) false false)
            (`SceneComponent.K2_SetWorldLocation` (`/Game/01_Blueprints/BP_ElevatorDoors.DoorR` _childdoortop_2) (`KismetMathLibrary.VLerp` (`SceneComponent.K2_GetComponentLocation` (`/Game/01_Blueprints/BP_ElevatorDoors.DoorR_Out` _childdoortop_2)) (`SceneComponent.K2_GetComponentLocation` (`/Game/01_Blueprints/BP_ElevatorDoors.DoorR_In` _childdoortop_2)) _lerpprog) false false))))
      (:`Finished`
        (`KismetSystemLibrary.PrintString` "Door closed")
        (set `self.DoorsOpen` false)))
    (else
      ;;[1 1 1] Opoening Doors
      (bind (_direction_2 _lerpval) (`Timeline|DoorOpen` :!via `PlayFromStart`)
        (:`Update`
          (`SceneComponent.K2_SetWorldLocation` (`self.DoorL`) (`KismetMathLibrary.VLerp` (`SceneComponent.K2_GetComponentLocation` (`self.DoorL_In`)) (`SceneComponent.K2_GetComponentLocation` (`self.DoorL_Out`)) _lerpval) false false)
          (`SceneComponent.K2_SetWorldLocation` (`self.DoorR`) (`KismetMathLibrary.VLerp` (`SceneComponent.K2_GetComponentLocation` (`self.DoorR_In`)) (`SceneComponent.K2_GetComponentLocation` (`self.DoorR_Out`)) _lerpval) false false)
          (if (`self.AtBottom`)
            (`SceneComponent.K2_SetWorldLocation` (`/Game/01_Blueprints/BP_ElevatorDoors.DoorL` _childdoorbottom_2) (`KismetMathLibrary.VLerp` (`SceneComponent.K2_GetComponentLocation` (`/Game/01_Blueprints/BP_ElevatorDoors.DoorL_In` _childdoorbottom_2)) (`SceneComponent.K2_GetComponentLocation` (`/Game/01_Blueprints/BP_ElevatorDoors.DoorL_Out` _childdoorbottom_2)) _lerpval) false false)
            (`SceneComponent.K2_SetWorldLocation` (`/Game/01_Blueprints/BP_ElevatorDoors.DoorR` _childdoorbottom_2) (`KismetMathLibrary.VLerp` (`SceneComponent.K2_GetComponentLocation` (`/Game/01_Blueprints/BP_ElevatorDoors.DoorR_In` _childdoorbottom_2)) (`SceneComponent.K2_GetComponentLocation` (`/Game/01_Blueprints/BP_ElevatorDoors.DoorR_Out` _childdoorbottom_2)) _lerpval) false false)
            (else
              (`SceneComponent.K2_SetWorldLocation` (`/Game/01_Blueprints/BP_ElevatorDoors.DoorL` _childdoortop) (`KismetMathLibrary.VLerp` (`SceneComponent.K2_GetComponentLocation` (`/Game/01_Blueprints/BP_ElevatorDoors.DoorL_In` _childdoortop)) (`SceneComponent.K2_GetComponentLocation` (`/Game/01_Blueprints/BP_ElevatorDoors.DoorL_Out` _childdoortop)) _lerpval) false false)
              (`SceneComponent.K2_SetWorldLocation` (`/Game/01_Blueprints/BP_ElevatorDoors.DoorR` _childdoortop) (`KismetMathLibrary.VLerp` (`SceneComponent.K2_GetComponentLocation` (`/Game/01_Blueprints/BP_ElevatorDoors.DoorR_In` _childdoortop)) (`SceneComponent.K2_GetComponentLocation` (`/Game/01_Blueprints/BP_ElevatorDoors.DoorR_Out` _childdoortop)) _lerpval) false false))))
        (:`Finished`
          (`KismetSystemLibrary.PrintString` "Door Opened")
          (set `self.DoorsOpen` true))))))

(fn `UserConstructionScript`)