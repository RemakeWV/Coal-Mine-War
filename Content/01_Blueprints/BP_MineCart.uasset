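; BP_MineCart is a rideable mine cart that carries a player along a spline track.
; Activate fires only while the cart is not moving and, if it is active, locks the player to PlayerHolder.
; A timeline, scaled by Duration and started at CartStartOffset, moves and rotates the cart along TrackReference's spline by distance.
; When it finishes, the player is released at ExitPoint, but IsMoving is never reset.
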(event `/Game/01_Blueprints/Data/iInteractable.Activate`
  (params (Player :type "/Game/01_Blueprints/BP_Player Object Reference"))
  (if (not (`self.IsMoving`))
    (set `self.IsMoving` true)
    (if (`self.ActiveCart`)
      (set `self.ActivatedPlayer` Player)
      ;[1 1 1] Puts player in Cart
      (`/Game/01_Blueprints/BP_Player.Lock to Place` (`self.ActivatedPlayer`) (`SceneComponent.K2_GetComponentLocation` (`self.PlayerHolder`)) (`self.PlayerHolder`))
      (`self.MoveCart`))))

(event `MoveCart`
  (bind _cartmover_timeline (`self.CartMover_Timeline`))
  (bind _spline (`/Game/01_Blueprints/Splines/BP_SplineActor.Spline` (`self.TrackReference`)))
  (bind _returnvalue (`KismetMathLibrary.Lerp` 0.0 (`SplineComponent.GetSplineLength` _spline) (`self.Alpha`)))
  (`TimelineComponent.SetPlayRate` _cartmover_timeline (/ 1.0 (`self.Duration`)))
  (`TimelineComponent.SetNewTime` _cartmover_timeline (`self.CartStartOffset`))
  (bind (_direction _alpha) (`Timeline|CartMover_Timeline`)
    (:`Update`
      (set `self.Alpha` _alpha)
      (`self.K2_SetActorLocationAndRotation` (`SplineComponent.GetLocationAtDistanceAlongSpline` _spline _returnvalue "World") (`SplineComponent.GetRotationAtDistanceAlongSpline` _spline _returnvalue "World")))
    (:`Finished`
      (`/Game/01_Blueprints/BP_Player.UnlockToPlace` (`self.ActivatedPlayer`) (`SceneComponent.K2_GetComponentLocation` (`self.Exit point`))))))

(fn `UserConstructionScript`)