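; Rusted lantern Blueprint that continuously varies the intensity of its point light as a flicker effect.
; BeginPlay starts an endless loop with two tiny random delays, each shorter than a typical frame, instead of using Tick.
; Each pass picks a random target intensity and lerps the current value toward it by a minuscule random alpha, so changes are heavily damped and frame-rate dependent.
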(event `self.ReceiveBeginPlay`
  (bind _returnvalue (`KismetMathLibrary.RandomFloatInRange` 0.0001 0.0005))
  (bind _pointlight (`self.PointLight`))
  (`KismetSystemLibrary.Delay` _returnvalue :!label _label)
  (bind _output_get (set `self.FlickerIntensity` (`KismetMathLibrary.RandomFloatInRange` 800.0 5000.0)))
  (`LightComponent.SetIntensity` _pointlight (`KismetMathLibrary.Lerp` (`LightComponentBase.Intensity` _pointlight) _output_get (/ _returnvalue 2.0)))
  (`KismetSystemLibrary.Delay` (`KismetMathLibrary.RandomFloatInRange` 0.0001 0.0005))
  (goto _label))

(fn `UserConstructionScript`)