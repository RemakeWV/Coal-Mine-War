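; Floor-cleaning bot that roams the NavMesh and removes Trash actors it bumps into.
; A looping timer turns it slightly, then AI-moves it to random nearby points.
; Overlapping Trash while idle, with no valid prior target, pauses wandering to approach it, resuming only on move success.
; Hitting Trash plays a timeline that shrinks its mesh, then destroys it; the pull-toward-bot movement is disconnected.
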(event `self.ReceiveHit`
  (params (MyComp :type "PrimitiveComponent Object Reference") (Other :type "Actor Object Reference") (OtherComp :type "PrimitiveComponent Object Reference") (bSelfMoved :type Boolean) (HitLocation :type "Vector Structure") (HitNormal :type "Vector Structure") (NormalImpulse :type "Vector Structure") (Hit :type "HitResult Structure (by ref)"))
  (bind _astrash (cast `/Game/01_Blueprints/Trash` Other))
  (bind (_direction _newtrack_0) (`Timeline|Shrink` :!via `PlayFromStart`)
    (:`Update`
      (`SceneComponent.SetWorldScale3D` (`StaticMeshActor.StaticMeshComponent` _astrash) (`KismetMathLibrary.VLerp` (0.146671 0.146671 0.146671) (0.0 0.0 0.0) _newtrack_0)))
    (:`Finished`
      (`self.K2_DestroyActor` _astrash))))

(event `self.ReceiveActorBeginOverlap`
  (params (OtherActor :type "Actor Object Reference"))
  (if (not (`self.IsMoving?`))
    (bind _astrash (cast `/Game/01_Blueprints/Trash` OtherActor))
    (`self.LastSeenTrash`
      (:`then`)
      (:`else`
        (set `self.LastSeenTrash` _astrash)
        (`KismetSystemLibrary.K2_ClearAndInvalidateTimerHandle` (`self.RandomMoveTimer`))
        (set `self.IsMoving?` true)
        (`|AIMoveTo` self (0.0 0.0 0.0) (`self.LastSeenTrash`) 10.0
          (:`OnSuccess`
            (set `self.IsMoving?` false)
            (bind _returnvalue (`KismetSystemLibrary.K2_SetTimerDelegate` (delegate `GoToRandomPoint`) 10.0 true :!label _label))
            (`self.GoToRandomPoint`)
            (set `self.RandomMoveTimer` _returnvalue)))))))

(event `self.ReceiveBeginPlay`
  (goto _label))

(event `GoToRandomPoint`
  (bind _capsulecomponent (`self.CapsuleComponent`))
  (bind _randomlocation (`NavigationSystemV1.K2_GetRandomLocationInNavigableRadius` (`SceneComponent.K2_GetComponentLocation` (`self.CapsuleComponent`)) 1000.0 null null))
  (bind (_returnvalue_roll _returnvalue_pitch _returnvalue_yaw) (`KismetMathLibrary.BreakRotator` (`KismetMathLibrary.FindLookAtRotation` (`SceneComponent.K2_GetComponentLocation` _capsulecomponent) _randomlocation)))
  (`self.K2_SetActorRotation` (`KismetMathLibrary.RInterpTo` (`SceneComponent.K2_GetComponentRotation` _capsulecomponent) (`KismetMathLibrary.MakeRotator` _returnvalue_roll 0.0 _returnvalue_yaw) (* (`GameplayStatics.GetWorldDeltaSeconds`) 0.001) 5.0))
  (`KismetSystemLibrary.Delay` 1.0)
  (`|AIMoveTo` self _randomlocation null))

(fn `UserConstructionScript`)