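; BP_BFL is a Blueprint function library of shared helpers for saving, settings, UI audio and controller icons.
; Save, load and settings lookups cast the game instance to GameInfo and call its save and load functions or read PlayerSettingsInfo.
; Audio helpers derive volume from those settings, scaling master volume by effects volume for the button press sound or by voice volume for voice.
; GetIcon maps a controller type to an entry in a list of possible icons.
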(fn `GetIcon`
  (params (Controller :type "/Game/01_Blueprints/Data/ControllerType Enum" :default "NewEnumerator0"))
  (returns (Icon :type "Texture2D Object Reference"))
  (locals (PossibleIcons :type "Array of Texture2D Object Reference") (IconIndex :type Integer :default 0))
  (switch `/Game/01_Blueprints/Data/ControllerType` Controller
    (:`NewEnumerator0`
      (set `local.IconIndex` 0))
    (:`NewEnumerator1`
      (set `local.IconIndex` 1))
    (:`NewEnumerator2`
      (set `local.IconIndex` 2))
    (:`NewEnumerator3`
      (set `local.IconIndex` 3)))
  (return (`|GetArrayItem` (`local.PossibleIcons`) (`local.IconIndex`))))

(fn `LoadGame`
  (bind _asgame_info (cast `/Game/01_Blueprints/Data/GameInfo` (`GameplayStatics.GetGameInstance` null)))
  (`/Game/01_Blueprints/Data/GameInfo.LoadGame` _asgame_info))

(fn `PlayButtonPressSound`
  (bind ((`MasterVolume_2_D8470D7A40A84D4DFD05EBB7D7858A40` _mastervolume) (`EffectsVolume_12_DED82C854828897FEF948DA11A2E5071` _effectsvolume)) (break `/Game/01_Blueprints/Data/PlayerSettings` (`self.ReturnSettings` null)))
  (`GameplayStatics.PlaySound2D` null "/Game/06_Sounds/ButtonPress_Cue.ButtonPress_Cue" (* _mastervolume _effectsvolume) 1.0 0.0 null null))

(fn `ReturnSettings`
  (returns (PlayerSettingsInfo :type "/Game/01_Blueprints/Data/PlayerSettings Structure"))
  (bind _asgame_info (cast `/Game/01_Blueprints/Data/GameInfo` (`GameplayStatics.GetGameInstance` null)))
  (return (`/Game/01_Blueprints/Data/GameInfo.PlayerSettingsInfo` _asgame_info)))

(fn `SaveGame`
  (bind _asgame_info (cast `/Game/01_Blueprints/Data/GameInfo` (`GameplayStatics.GetGameInstance` null)))
  (`/Game/01_Blueprints/Data/GameInfo.SaveGame` _asgame_info))

(fn `VoiceAudioSettings`
  (returns (Volume :type "Float (double-precision)"))
  (bind ((`MasterVolume_2_D8470D7A40A84D4DFD05EBB7D7858A40` _mastervolume) (`VoiceVolume_13_04D75AD64F9F213060E0C586C29E75AA` _voicevolume)) (break `/Game/01_Blueprints/Data/PlayerSettings` (`self.ReturnSettings` null)))
  (return (* _mastervolume _voicevolume)))