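; BP_GameInfo holds player settings, handles their saving and loading, and adjusts the player's height.
; SaveGame and LoadGame copy the settings to and from a SaveData object in the "Info" slot; saving creates one only when no save exists.
; Increase and Decrease Play Scale step BP_Player's capsule half-height within limits on the passed scale, shifting InWorldMenu vertically to match.
; ShowPauseMenu is an empty event.
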(event `ShowPauseMenu`
  (params (Player :type "/Game/01_Blueprints/BP_Player Object Reference")))

(fn `Decrease Play Scale`
  (params (PlayerScale :type "Float (double-precision)"))
  (returns (ActualPlayerHeight :type "Float (double-precision)"))
  (locals (PlayerHeight :type "Float (double-precision)"))
  (bind _output_get (set `local.PlayerHeight` PlayerScale))
  (if (not (<= _output_get 0.0))
    (bind _asbp_player (cast `/Game/01_Blueprints/BP_Player` (`GameplayStatics.GetPlayerCharacter` 0)))
    (bind _capsulecomponent (`Character.CapsuleComponent` _asbp_player))
    (bind _returnvalue (- (`CapsuleComponent.CapsuleHalfHeight` _capsulecomponent) 5.0))
    (`CapsuleComponent.SetCapsuleHalfHeight` _capsulecomponent _returnvalue true)
    (bind _returnvalue_2 (`GameplayStatics.GetActorOfClass` "/Game/01_Blueprints/In-WorldMenu.In-WorldMenu_C"))
    (`Actor.K2_AddActorWorldOffset` _returnvalue_2 (0.0 0.0 -5.0) false false)
    (return _returnvalue)))

(fn `Increase Play Scale`
  (params (PlayerScale :type "Float (double-precision)"))
  (returns (ActualPlayerHeight :type "Float (double-precision)"))
  (locals (PlayerHeight :type "Float (double-precision)"))
  (bind _output_get (set `local.PlayerHeight` PlayerScale))
  (if (not (>= _output_get 1.0))
    (bind _asbp_player (cast `/Game/01_Blueprints/BP_Player` (`GameplayStatics.GetPlayerCharacter` 0)))
    (bind _capsulecomponent (`Character.CapsuleComponent` _asbp_player))
    (bind _returnvalue (+ (`CapsuleComponent.CapsuleHalfHeight` _capsulecomponent) 5.0))
    (`CapsuleComponent.SetCapsuleHalfHeight` _capsulecomponent _returnvalue true)
    (bind _returnvalue_2 (`GameplayStatics.GetActorOfClass` "/Game/01_Blueprints/In-WorldMenu.In-WorldMenu_C"))
    (`Actor.K2_AddActorWorldOffset` _returnvalue_2 (0.0 0.0 5.0) false false)
    (return _returnvalue)))

(fn `LoadGame`
  (returns (SaveData :type "/Game/01_Blueprints/Data/SaveData Object Reference"))
  (bind _returnvalue (`GameplayStatics.LoadGameFromSlot` "Info"))
  (bind _assave_data (cast `/Game/01_Blueprints/Data/SaveData` _returnvalue))
  (bind _output_get (set `self.SaveDataFIle` _assave_data))
  (set `self.PlayerSettingsInfo` (`/Game/01_Blueprints/Data/SaveData.PlayerSettingsSave` _output_get))
  (return _output_get))

(fn `SaveGame`
  (bind _returnvalue (`GameplayStatics.DoesSaveGameExist` "Info"))
  (if (not _returnvalue)
    (bind _returnvalue_2 (`GameplayStatics.CreateSaveGameObject` "/Game/01_Blueprints/Data/SaveData.SaveData_C"))
    (bind _output_get (set `self.SaveDataFIle` _returnvalue_2)))
  (set `/Game/01_Blueprints/Data/SaveData.PlayerSettingsSave` (`self.PlayerSettingsInfo`) _output_get)
  (`GameplayStatics.SaveGameToSlot` (`self.SaveDataFIle`) "Info"))