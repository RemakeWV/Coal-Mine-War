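; VR player Blueprint that teleports the player to a spot aimed at with the right motion controller.
; Once CheckTeleport is pressed, Tick line-traces from the controller each frame; TriggerHeld is never cleared on release.
; Near-flat hits are projected to the navigation mesh and marked with a debug cylinder.
; The Teleport input then moves the actor there, adding the HMD camera's horizontal relative offset.
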(event `InputAction|CheckTeleport`
  (params (Key :type "Key Structure"))
  (:`Pressed`
    (set `self.TriggerHeld` true))
  (:`Released`
    (set `self.Teleport` false)))

(event `InputAction|Teleport`
  (params (Key :type "Key Structure"))
  (:`Pressed`
    (if (and (`self.TriggerHeld`) (`self.Teleport`))
      (`self.TeleportToDestination` (`self.TeleportLoc`)))))

(event `self.ReceiveTick`
  (params (DeltaSeconds :type "Float (single-precision)"))
  (bind _motioncontroller_right (`self.MotionController-Right`))
  (if (`self.TriggerHeld`)
    (`self.GetDestination` (`SceneComponent.K2_GetComponentLocation` _motioncontroller_right) (`SceneComponent.GetForwardVector` _motioncontroller_right))))

(fn `GetDestination`
  (params (Position :type "Vector Structure") (ForwardVector :type "Vector Structure"))
  (bind _outhit (`KismetSystemLibrary.LineTraceSingle` Position (+ Position (* ForwardVector 10000.0)) "TraceTypeQuery1"))
  (bind (_bblockinghit _binitialoverlap _time _distance _location _impactpoint _normal) (`GameplayStatics.BreakHitResult` _outhit))
  (bind _output_get (set `self.Teleport` (> (`KismetMathLibrary.Dot_VectorVector` _normal (0.0 0.0 1.0)) 0.9)))
  (if _output_get
    (bind _output_get_2 (set `self.TeleportLoc` (`NavigationSystemV1.K2_ProjectPointToNavigation` _location)))
    (`KismetSystemLibrary.DrawDebugCylinder` _output_get_2 (+ _output_get_2 (* _normal 10.0)) 50.0 12 (struct :`G` 1.0 :`B` 0.055177 :`A` 1.0) 0.0 1.0)))

(fn `TeleportToDestination`
  (params (Location :type "Vector Structure"))
  (bind (_relativelocation_x _relativelocation_y) (`KismetMathLibrary.BreakVector` (`SceneComponent.RelativeLocation` (`self.HMD-Camera`))))
  (`self.K2_SetActorLocation` (+ Location (`KismetMathLibrary.MakeVector` _relativelocation_x _relativelocation_y))))

(fn `UserConstructionScript`)