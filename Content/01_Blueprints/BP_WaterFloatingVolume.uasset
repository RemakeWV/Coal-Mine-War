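; Water floating volume that suspends gravity for items and the player inside its box.
; Each tick it polls overlaps, turns off gravity on physics-simulating item meshes and adds a small +X velocity, so the drift accumulates per frame.
; It also turns off gravity on the player's capsule, without pushing it.
; End overlap restores gravity for both and zeroes the item's linear velocity.
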(event `self.ReceiveActorEndOverlap`
  (params (OtherActor :type "Actor Object Reference"))
  (bind _asbp_item (cast `/Game/01_Blueprints/Items/BP_Item` OtherActor)
    (:`then`
      (bind _staticmesh (`/Game/01_Blueprints/Items/BP_Item.StaticMesh` _asbp_item))
      (`PrimitiveComponent.SetEnableGravity` _staticmesh true)
      (`PrimitiveComponent.SetPhysicsLinearVelocity` _staticmesh (0.0 0.0 0.0) false "None"))
    (:`CastFailed`
      (bind _asbp_player (cast `/Game/01_Blueprints/BP_Player` OtherActor))
      (`PrimitiveComponent.SetEnableGravity` (`Character.CapsuleComponent` _asbp_player) true))))

(event `self.ReceiveTick`
  (params (DeltaSeconds :type "Float (single-precision)"))
  (bind _overlappingactors (`PrimitiveComponent.GetOverlappingActors` (`self.Box`) "/Game/01_Blueprints/Items/BP_Item.BP_Item_C"))
  (bind _overlappingactors_2 (`PrimitiveComponent.GetOverlappingActors` (`self.Box`) "/Game/01_Blueprints/BP_Player.BP_Player_C"))
  (`|ExecutionSequence`
    (:`then_0`
      (if (> (`KismetArrayLibrary.Array_Length` _overlappingactors) 0)
        (for _array_element _overlappingactors
          (bind _asbp_item (cast `/Game/01_Blueprints/Items/BP_Item` _array_element))
          (bind _staticmesh (`/Game/01_Blueprints/Items/BP_Item.StaticMesh` _asbp_item))
          (if (`SceneComponent.IsSimulatingPhysics` _staticmesh "None")
            (`PrimitiveComponent.SetEnableGravity` _staticmesh false)
            (`PrimitiveComponent.SetPhysicsLinearVelocity` _staticmesh (0.5 0.0 0.0) true "None")))))
    (:`then_1`
      (if (> (`KismetArrayLibrary.Array_Length` _overlappingactors_2) 0)
        (for _array_element_2 _overlappingactors_2
          (bind _asbp_player (cast `/Game/01_Blueprints/BP_Player` _array_element_2))
          (`PrimitiveComponent.SetEnableGravity` (`Character.CapsuleComponent` _asbp_player) false))))))

(fn `UserConstructionScript`)