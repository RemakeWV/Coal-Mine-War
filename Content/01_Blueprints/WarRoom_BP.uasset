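; War room actor that switches the game from the museum to the mine war battle when BP_Player overlaps it.
; BeginPlay applies one dynamic M_Dissolve material to its six static meshes.
; The overlap calls StartSim, which unloads five museum stream levels and loads MineWar_Battle with a blocking load.
; It also plays the Dissolve timeline from the start, driving the shared material's dissolve amount to fade all six meshes together.
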(event `self.ReceiveBeginPlay`
  (bind _returnvalue (`KismetMaterialLibrary.CreateDynamicMaterialInstance` "/Game/04_Materials/M_Dissolve.M_Dissolve"))
  (bind _output_get (set `self.DynamicMaterial` _returnvalue))
  (`PrimitiveComponent.SetMaterial` (`self.StaticMesh1`) 0 _output_get)
  (`PrimitiveComponent.SetMaterial` (`self.StaticMesh2`) 0 _output_get)
  (`PrimitiveComponent.SetMaterial` (`self.StaticMesh3`) 0 _output_get)
  (`PrimitiveComponent.SetMaterial` (`self.StaticMesh4`) 0 _output_get)
  (`PrimitiveComponent.SetMaterial` (`self.StaticMesh`) 0 _output_get)
  (`PrimitiveComponent.SetMaterial` (`self.StaticMesh5`) 0 _output_get))

(event `StartSim`
  (bind _museum_level_names (`self.Museum_Level_Names`))
  (`|ExecutionSequence`
    (:`then_0`
      (`GameplayStatics.UnloadStreamLevel` (`|GetArrayItem` _museum_level_names)))
    (:`then_1`
      (`GameplayStatics.UnloadStreamLevel` (`|GetArrayItem` _museum_level_names 1)))
    (:`then_2`
      (`GameplayStatics.UnloadStreamLevel` (`|GetArrayItem` _museum_level_names 2)))
    (:`then_3`
      (`GameplayStatics.UnloadStreamLevel` (`|GetArrayItem` _museum_level_names 3)))
    (:`then_4`
      (`GameplayStatics.UnloadStreamLevel` (`|GetArrayItem` _museum_level_names 4)))
    (:`then_5`
      (`GameplayStatics.LoadStreamLevel` "MineWar_Battle" true true))))

(event `self.ReceiveActorBeginOverlap`
  (params (OtherActor :type "Actor Object Reference"))
  (cast `/Game/01_Blueprints/Player/BP_Player` OtherActor)
  (`self.StartSim`)
  (bind (_direction _newtrack_0) (`Timeline|Dissolve` :!via `PlayFromStart`)
    (:`Update`
      (`MaterialInstanceDynamic.SetScalarParameterValue` (`self.DynamicMaterial`) "Dissolve Amount" (`KismetMathLibrary.Lerp` 0.0 1.0 _newtrack_0)))))

(fn `UserConstructionScript`)