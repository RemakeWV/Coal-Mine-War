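; World-space exhibit info panel actor that shows a title, description, picture info and image and turns toward the player.
; The construction script looks up the row for the selected Exhibit enum in the ExhibitList data table and caches it as Info.
; On BeginPlay, UpdateInfo passes that data to the TestWidget in its widget component.
; Each Tick applies only look-at yaw and roll toward a point slightly above the player character, leaving out pitch.
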(event `self.ReceiveBeginPlay`
  (bind (_info_title _info_description _info_imageinfo _info_image) (break `/Game/01_Blueprints/Data/ExhibitStruct` (`self.Info`)))
  (`self.UpdateInfo` _info_title _info_description _info_imageinfo _info_image))

(event `self.ReceiveTick`
  (params (DeltaSeconds :type "Float (single-precision)"))
  (bind (_returnvalue_roll _returnvalue_pitch _returnvalue_yaw) (`KismetMathLibrary.BreakRotator` (`KismetMathLibrary.FindLookAtRotation` (`self.K2_GetActorLocation`) (+ (`self.K2_GetActorLocation` (`GameplayStatics.GetPlayerCharacter` 0)) (0.0 0.0 25.0)))))
  (`self.K2_SetActorRotation` (`KismetMathLibrary.MakeRotator` _returnvalue_roll 0.0 _returnvalue_yaw) true))

(event `UpdateInfo`
  (params (Title :type String) (Description :type String) (PictureInfo :type String) (Image :type "Texture2D Object Reference"))
  (bind _astest_widget (cast `/Game/09_UI/TESTUI/TestWidget` (`WidgetComponent.GetUserWidgetObject` (`self.Widget`))))
  (`/Game/09_UI/TESTUI/TestWidget.UpdateTexts` _astest_widget Title Description PictureInfo Image))

(fn `UserConstructionScript`
  (bind _returnvalue (`|GetDataTableRow` "/Game/01_Blueprints/Data/ExhibitList.ExhibitList" (`KismetStringLibrary.Conv_StringToName` (`|GetEnumeratorNameAsString` (`self.Exhibit`))))
    (:`then`
      (set `self.Info` _returnvalue))))