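; BP_Weapon is a weapon actor in the WW2_M1928 content that appears to serve as a base for specific weapons.
; Its construction script applies a configurable anim instance class and skeletal mesh to WeaponMesh.
; BeginPlay caches player 0's pawn as OwnerPawn.
; Ammo extraction, query and reload functions are placeholders returning false, zero or nothing, with no ammo logic here.
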(event `self.ReceiveBeginPlay`
  (set `self.OwnerPawn` (`GameplayStatics.GetPlayerPawn` 0)))

(fn `ExtractAmmo`
  (returns (isEmpty :type Boolean))
  (return false))

(fn `GetCurrentAmmo`
  (returns (remainAmmo :type Integer) (isFullReloaded :type Boolean))
  (return 0 false))

(fn `ReloadAmmo`)

(fn `UserConstructionScript`
  (bind _weaponmesh (`self.WeaponMesh`))
  (`SkeletalMeshComponent.SetAnimInstanceClass` _weaponmesh (`self.WeaponAnimBP`))
  (`SkinnedMeshComponent.SetSkinnedAssetAndUpdate` _weaponmesh (`self.VisibleWeaponMesh`) true))