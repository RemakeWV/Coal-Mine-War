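; Child weapon Blueprint for the M1928 that switches between two variants, M1928A1 and M1928 Drum, each with its own ammo count.
; Changing type swaps the skeletal mesh and AnimBP on the weapon mesh without resetting either count.
; Both counts fill on BeginPlay; extracting, reloading and querying ammo act on the current type, reporting empty or full state.
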(event `self.ReceiveBeginPlay`
  (`parent.ReceiveBeginPlay`)
  (set `self.M1928A1_CurrentAmmo` (`self.M1928A1_MaxAmmo`))
  (set `self.M1928Drum_CurrentAmmo` (`self.M1928Drum_MaxAmmo`)))

(event `self.ReloadAmmo`
  (switch `/Game/WW2_M1928/Blueprints/M1928Type` (`self.CurrentWeaponType`)
    (:`NewEnumerator0`
      (set `self.M1928A1_CurrentAmmo` (`self.M1928A1_MaxAmmo`)))
    (:`NewEnumerator1`
      (set `self.M1928Drum_CurrentAmmo` (`self.M1928Drum_MaxAmmo`)))))

(fn `ChangeAnotherType`
  (params (ChangeWeaponType :type "/Game/WW2_M1928/Blueprints/M1928Type Enum" :default "NewEnumerator0"))
  (bind _weaponmesh (`self.WeaponMesh`))
  (set `self.CurrentWeaponType` ChangeWeaponType)
  (`SkinnedMeshComponent.SetSkinnedAssetAndUpdate` _weaponmesh (select `/Game/WW2_M1928/Blueprints/M1928Type` ChangeWeaponType :`NewEnumerator0` "/Game/WW2_M1928/Weapons/Meshes/SK_M1928A1.SK_M1928A1" :`NewEnumerator1` "/Game/WW2_M1928/Weapons/Meshes/SK_M1928.SK_M1928" :!type "SkeletalMesh Object Reference") true)
  (`SkeletalMeshComponent.SetAnimInstanceClass` _weaponmesh (select `/Game/WW2_M1928/Blueprints/M1928Type` ChangeWeaponType :`NewEnumerator0` "/Game/WW2_M1928/Weapons/Anims_Gun/Gun_M1928A1/M1928A_AnimBP.M1928A_AnimBP_C" :`NewEnumerator1` "/Game/WW2_M1928/Weapons/Anims_Gun/Gun_M1928/M1928Drum_AnimBP.M1928Drum_AnimBP_C" :!type "Object Class Reference")))

(fn `ExtractAmmo`
  (returns (isEmpty :type Boolean))
  (locals (emptyState :type Boolean))
  (switch `/Game/WW2_M1928/Blueprints/M1928Type` (`self.CurrentWeaponType`)
    (:`NewEnumerator0`
      (bind _output_get (set `self.M1928A1_CurrentAmmo` (- (`self.M1928A1_CurrentAmmo`) 1)))
      (set `local.emptyState` (<= _output_get 0)))
    (:`NewEnumerator1`
      (bind _output_get_2 (set `self.M1928Drum_CurrentAmmo` (- (`self.M1928Drum_CurrentAmmo`) 1)))
      (set `local.emptyState` (<= _output_get_2 0))))
  (return (`local.emptyState`)))

(fn `GetCurrentAmmo`
  (returns (remainAmmo :type Integer) (isFullReloaded :type Boolean))
  (locals (FullAmmo :type Boolean :default false))
  (bind _currentweapontype (`self.CurrentWeaponType`))
  (bind _m1928drum_currentammo (`self.M1928Drum_CurrentAmmo`))
  (bind _m1928a1_currentammo (`self.M1928A1_CurrentAmmo`))
  (switch `/Game/WW2_M1928/Blueprints/M1928Type` _currentweapontype
    (:`NewEnumerator0`
      (set `local.FullAmmo` (== (`self.M1928A1_MaxAmmo`) _m1928a1_currentammo)))
    (:`NewEnumerator1`
      (set `local.FullAmmo` (== (`self.M1928Drum_MaxAmmo`) _m1928drum_currentammo))))
  (return (select `/Game/WW2_M1928/Blueprints/M1928Type` _currentweapontype :`NewEnumerator0` _m1928a1_currentammo :`NewEnumerator1` _m1928drum_currentammo) (`local.FullAmmo`)))

(fn `UserConstructionScript`
  (`parent.UserConstructionScript`))