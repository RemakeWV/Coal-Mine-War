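; ThunderStorm_BP drives a looping thunderstorm effect, with lightning flashes followed by thunder, from the title screen sound folder.
; On BeginPlay it waits a random interval, then briefly spikes LightingSkyLight intensity in a burst of randomly spaced flashes.
; When the burst reaches its random flash count, it plays a 2D thunder cue, rerolls the count and repeats the cycle indefinitely.
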(event `self.ReceiveBeginPlay`
  (bind _lightingskylight (`self.LightingSkyLight`))
  (set `self.MaxFlashes` (`KismetMathLibrary.RandomIntegerInRange` 1 6))
  (`KismetSystemLibrary.Delay` (`KismetMathLibrary.RandomFloatInRange` 10.0 45.0) :!label _label)
  (if (>= (`self.FlashesCount`) (`self.MaxFlashes`)) :!label _label_2
    (`GameplayStatics.PlaySound2D` "/Game/06_Sounds/TitleScreen/Thunder_A_Cue.Thunder_A_Cue" 1.0 1.0 0.0 null null)
    (set `self.FlashesCount` 0)
    (set `self.MaxFlashes` 0)
    (set `self.MaxFlashes` (`KismetMathLibrary.RandomIntegerInRange` 1 6))
    (goto _label)
    (else
      (`SkyLightComponent.SetIntensity` _lightingskylight 200.0)
      (`KismetSystemLibrary.Delay` 0.1)
      (`SkyLightComponent.SetIntensity` _lightingskylight 2.5)
      (`/Engine/EditorBlueprintResources/StandardMacros.IncrementInt` (`self.FlashesCount`)
        (:`  `
          (`KismetSystemLibrary.Delay` (`KismetMathLibrary.RandomFloatInRange` 0.01 0.15))
          (goto _label_2))))))

(fn `UserConstructionScript`)